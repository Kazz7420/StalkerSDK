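; Light fixture Blueprint that applies color and radius presets from data tables to its lights, emissive meshes and light beams.
; Construction merges both preset rows, sets lights, builds dynamic materials for tagged meshes and rotates tagged projector bases.
; Events swap glass materials on or off and drive flicker on emissives, beams and decals from light intensity.
; Further events override main-light parameters and shape a decal faking inner light from the spotlight.
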(event `OnConstruction_Child`
  (`self.GlassEmissive` (`self.IsEnabled`)))

(event `self.GlassEmissive`
  (params (OnOff :type Boolean))
  (bind _glowobjectsmaterialnew (`self.GlowObjectsMaterialNew`))
  (bind _glowobjectsmaterialorigin (`self.GlowObjectsMaterialOrigin`))
  ;[1 1 1] Emissive On/Off
  (if OnOff
    ;;[1 1 1] Dynamic Materials
    (bind _keys (`BlueprintMapLibrary.Map_Keys` _glowobjectsmaterialnew))
    (for _array_element _keys
      (`/Engine/EditorBlueprintResources/StandardMacros.IsValid` _array_element
        (:`Is Valid`
          (`PrimitiveComponent.SetMaterial` _array_element 0 (`BlueprintMapLibrary.Map_Find` _glowobjectsmaterialnew _array_element)))))
    (else
      (bind _keys_2 (`BlueprintMapLibrary.Map_Keys` _glowobjectsmaterialorigin))
      (for _array_element_2 _keys_2
        (`/Engine/EditorBlueprintResources/StandardMacros.IsValid` _array_element_2
          (:`Is Valid`
            (`PrimitiveComponent.SetMaterial` _array_element_2 0 (`BlueprintMapLibrary.Map_Find` _glowobjectsmaterialorigin _array_element_2))))))))

(event `self.GlassEmissiveFlick`
  (params (LightIntensity :type "Float (double-precision)"))
  (bind _returnvalue (>= LightIntensity 0.1))
  (bind (_presetvalue_presetname _presetvalue_intensity _presetvalue_lightcolor _presetvalue_attenuationradius _presetvalue_temperature _presetvalue_emissivecolor _presetvalue_emissivebrightness _presetvalue_emissivepower _presetvalue_lightbeamcolor _presetvalue_lightbeambrightness) (break `/Game/_STALKER2/GameDesign/InteractiveObjects/LightBulb/DT_LightPresets/S_LightPresset` (`self.PresetValue`)))
  (bind (_presetvalue_presetname_2 _presetvalue_intensity_2 _presetvalue_lightcolor_2 _presetvalue_attenuationradius_2 _presetvalue_temperature_2 _presetvalue_emissivecolor_2 _presetvalue_emissivebrightness_2) (break `/Game/_STALKER2/GameDesign/InteractiveObjects/LightBulb/DT_LightPresets/S_LightPresset` (`self.PresetValue`)))
  ;[1 1 1] Emissive Flickering
  (`|ExecutionSequence`
    (:`then_0`
      (bind _values (`BlueprintMapLibrary.Map_Values` (`self.GlowObjectsMaterialNew`)))
      (for _array_element _values
        (`/Engine/EditorBlueprintResources/StandardMacros.IsValid` _array_element
          (:`Is Valid`
            (if _returnvalue
              (`MaterialInstanceDynamic.SetScalarParameterValue` _array_element "EmissiveMult" _presetvalue_emissivebrightness_2)
              ;;[0.2138 0.5806 1] New Material Emission
              (`MaterialInstanceDynamic.SetScalarParameterValue` _array_element "EmissiveIntensity" (`KismetMathLibrary.FClamp` _presetvalue_emissivebrightness_2))
              (else
                (`MaterialInstanceDynamic.SetScalarParameterValue` _array_element "EmissiveMult" 0.1)
                (`MaterialInstanceDynamic.SetScalarParameterValue` _array_element "EmissiveIntensity" 0.1))))))
      ;[1 1 1] LightBeam Flickering
      (for _array_element_2 (`self.LightBeamsDIM`)
        (`/Engine/EditorBlueprintResources/StandardMacros.IsValid` _array_element_2
          (:`Is Valid`
            (`MaterialInstanceDynamic.SetScalarParameterValue` _array_element_2 "LightBeamMult" (* _presetvalue_lightbeambrightness LightIntensity))))))
    (:`then_1`
      ;[1 1 1] Decal fake Inner light Flicker
      (for _array_element_3 (`self.GetComponentsByTag` "/Script/Engine.DecalComponent" "Decal_fake_Inner_light")
        (`SceneComponent.SetVisibility` _array_element_3 (`SceneComponent.bVisible` _array_element_3) false)
        (`SceneComponent.SetVisibility` _array_element_3 (>= LightIntensity 0.1) false)))
    (:`then_2`
      ;[1 1 1] Glow_Flicker
      (for _array_element_4 (`self.GetComponentsByTag` "/Script/Engine.StaticMeshComponent" "EmissiveGlow")
        (`SceneComponent.SetVisibility` _array_element_4 (>= LightIntensity 0.1) false)))
    (:`then_3`
      (for _array_element_5 (`self.GetComponentsByTag` "/Script/Engine.StaticMeshComponent" "EmissiveGlassOpaqueMax")
        (bind _returnvalue_2 (`PrimitiveComponent.CreateDynamicMaterialInstance` _array_element_5 0 (`PrimitiveComponent.GetMaterial` _array_element_5 0) "None"))
        (if _returnvalue
          (`MaterialInstanceDynamic.SetScalarParameterValue` _returnvalue_2 "EmissiveIntensity_Max" 10.0)
          (`MaterialInstanceDynamic.SetScalarParameterValue` _returnvalue_2 "FlickerMult" 1.0)
          (else
            (`MaterialInstanceDynamic.SetScalarParameterValue` _returnvalue_2 "EmissiveIntensity_Max" 0.2)
            (`MaterialInstanceDynamic.SetScalarParameterValue` _returnvalue_2 "FlickerMult" 0.1)))))
    (:`then_4`
      (for _array_element_6 (`self.GetComponentsByTag` "/Script/Engine.StaticMeshComponent" "FlickerEmissiveMonitor")
        (bind _returnvalue_3 (`PrimitiveComponent.CreateDynamicMaterialInstance` _array_element_6 1 (`PrimitiveComponent.GetMaterial` _array_element_6 1) "None"))
        (if _returnvalue
          (`MaterialInstanceDynamic.SetScalarParameterValue` _returnvalue_3 "FlickerMult" 1.0)
          (else
            (`MaterialInstanceDynamic.SetScalarParameterValue` _returnvalue_3 "FlickerMult" 0.1)))))))

(event `UpdateLightParameters`
  (params (AttenuationRadius :type "Float (double-precision)") (ShadowBias :type "Float (double-precision)") (ShadowSlopeBias :type "Float (double-precision)") (ContactShadowLength :type "Float (double-precision)") (LightFunctionMaterial :type "MaterialInterface Object Reference") (InnerConeAngle :type "Float (double-precision)") (OuterConeAngle :type "Float (double-precision)") (InnerIntensityMultiplier :type "Float (double-precision)" :default 0.0) (`Light Falloff Exponen` :type "Float (double-precision)" :default 7.0))
  (bind _returnvalue (`KismetMathLibrary.FClamp` ShadowSlopeBias 0.2))
  (bind _returnvalue_2 (`KismetMathLibrary.FClamp` ContactShadowLength 0.04 0.1))
  (bind _returnvalue_3 (`KismetMathLibrary.FClamp` ShadowBias 0.2))
  (bind _returnvalue_4 (!= AttenuationRadius 0.0))
  (bind _returnvalue_5 (!= LightFunctionMaterial null))
  (bind _returnvalue_6 (!= ShadowSlopeBias 0.0))
  (bind _returnvalue_7 (!= ContactShadowLength 0.0))
  (bind _returnvalue_8 (!= ShadowBias 0.0))
  (bind (_presetvalue_presetname _presetvalue_intensity) (break `/Game/_STALKER2/GameDesign/InteractiveObjects/LightBulb/DT_LightPresets/S_LightPresset` (`self.PresetValue`)))
  (bind _returnvalue_9 (* InnerIntensityMultiplier _presetvalue_intensity))
  (`|ExecutionSequence`
    (:`then_0`
      ;[1 1 1] Main Light Setup
      ;;[1 1 1] AttenuationRadius
      (for _array_element (`self.GetComponentsByTag` "/Script/Engine.PointLightComponent" "MainLight")
        (if _returnvalue_4
          (`LocalLightComponent.SetAttenuationRadius` _array_element AttenuationRadius))
        ;;[1 1 1] ShadowBias
        (if _returnvalue_8
          (`LightComponent.SetShadowBias` _array_element _returnvalue_3))
        ;;[1 1 1] ShadowSlopeBias
        (if _returnvalue_6
          (`LightComponent.SetShadowSlopeBias` _array_element _returnvalue))
        ;;[1 1 1] ContactShadowLength
        (if _returnvalue_7
          (set `LightComponent.ContactShadowLength` _returnvalue_2 _array_element))
        ;;[1 1 1] LightFunctionMaterial
        (if _returnvalue_5
          (`LightComponent.SetLightFunctionMaterial` _array_element LightFunctionMaterial)))
      (for _array_element_2 (`self.GetComponentsByTag` "/Script/Engine.SpotLightComponent" "MainLight")
        (if _returnvalue_4
          (`LocalLightComponent.SetAttenuationRadius` _array_element_2 AttenuationRadius))
        (if _returnvalue_8
          (`LightComponent.SetShadowBias` _array_element_2 _returnvalue_3))
        (if _returnvalue_6
          (`LightComponent.SetShadowSlopeBias` _array_element_2 _returnvalue))
        (if _returnvalue_7
          (set `LightComponent.ContactShadowLength` _returnvalue_2 _array_element_2))
        (if _returnvalue_5
          (`LightComponent.SetLightFunctionMaterial` _array_element_2 LightFunctionMaterial))))
    (:`then_1`
      ;;[1 1 1] SpotLight Inner/Outer Cone Angle
      (for _array_element_3 (`self.SpotLights`)
        (if (!= InnerConeAngle 0.0)
          (`SpotLightComponent.SetInnerConeAngle` _array_element_3 (`KismetMathLibrary.FClamp` InnerConeAngle 1.0 95.0)))
        (if (!= OuterConeAngle 0.0)
          (`SpotLightComponent.SetOuterConeAngle` _array_element_3 (`KismetMathLibrary.FClamp` OuterConeAngle 1.0 95.0)))))
    (:`then_2`
      ;[1 1 1] InnerIntensity
      (if (>= InnerIntensityMultiplier 0.0)
        (for _array_element_4 (`self.InnerPointLights`)
          (`LightComponent.SetIntensity` _array_element_4 _returnvalue_9))
        (for _array_element_5 (`self.InnerSpotLights`)
          (`LightComponent.SetIntensity` _array_element_5 _returnvalue_9))))
    (:`then_3`
      ;[1 1 1] Light Falloff Exponent
      (for _array_element_6 (`self.GetComponentsByTag` "/Script/Engine.PointLightComponent" "MainLight")
        (`PointLightComponent.SetLightFalloffExponent` _array_element_6 `Light Falloff Exponen`)))))

(event `UpdateDecalInnerLightParameters`
  (params (Intensity_Decal :type "Float (double-precision)" :default 1.0) (`ScaleDecal-Z` :type "Float (double-precision)" :default 0.03) (`OffsetDecal-Z` :type "Float (double-precision)" :default 2.5) (Lenght :type "Float (double-precision)" :default 0.25) (Fix_Rotate_Decal :type Boolean) (`Turn OF Decal` :type Boolean :default true) (`Use location` :type Boolean :default false))
  (bind (_presetvalue_presetname _presetvalue_intensity _presetvalue_lightcolor _presetvalue_attenuationradius _presetvalue_temperature _presetvalue_emissivecolor _presetvalue_emissivebrightness _presetvalue_emissivepower _presetvalue_lightbeamcolor _presetvalue_lightbeambrightness _presetvalue_lightbeampower _presetvalue_emissiveintensity) (break `/Game/_STALKER2/GameDesign/InteractiveObjects/LightBulb/DT_LightPresets/S_LightPresset` (`self.PresetValue`)))
  (bind _returnvalue (/ (* `ScaleDecal-Z` 100.0) 2.0))
  (bind _returnvalue_2 (`KismetMathLibrary.ClampVectorSize` (`KismetMathLibrary.Conv_DoubleToVector` (/ Lenght 0.52)) 0.05 5.0))
  ;[0.349 0.349 0.349] Decal fake Inner light
  (for _array_element (`self.GetComponentsByTag` "/Script/Engine.DecalComponent" "Decal_fake_Inner_light")
    (for _array_element_2 (`self.GetComponentsByTag` "/Script/Engine.SpotLightComponent" "MainLight")
      (if `Turn OF Decal`
        (`SceneComponent.SetVisibility` _array_element (`SceneComponent.bVisible` _array_element_2) false)
        (if `Use location`
          _
          (elif Fix_Rotate_Decal
            (`SceneComponent.K2_SetRelativeRotation` _array_element (struct :`Pitch` 90.0 :`Yaw` -90.0 :`Roll` -180.0) false false)
            (`SceneComponent.SetRelativeScale3D` _array_element (`KismetMathLibrary.MakeVector` `ScaleDecal-Z` (.y _returnvalue_2) (.z _returnvalue_2)))
            (`SceneComponent.K2_SetRelativeLocation` _array_element (`KismetMathLibrary.MakeVector` 0.0 0.0 (+ (* 2.56 _returnvalue) `OffsetDecal-Z`)) false false)
            (else
              (`SceneComponent.SetRelativeScale3D` _array_element (`KismetMathLibrary.MakeVector` `ScaleDecal-Z` (.y _returnvalue_2) (.z _returnvalue_2)))
              (`SceneComponent.K2_SetRelativeLocation` _array_element (`KismetMathLibrary.MakeVector` 0.0 (+ (* -2.56 _returnvalue) `OffsetDecal-Z`)) false false))))
        ;;[0 0 0] Material Instance
        (bind _returnvalue_3 (`DecalComponent.CreateDynamicMaterialInstance` _array_element))
        (`MaterialInstanceDynamic.SetVectorParameterValue` _returnvalue_3 "Color" (`LightComponentBase.GetLightColor` _array_element_2))
        (`MaterialInstanceDynamic.SetScalarParameterValue` _returnvalue_3 "Temperature" (`LightComponent.Temperature` _array_element_2))
        (`MaterialInstanceDynamic.SetScalarParameterValue` _returnvalue_3 "Multiply" (* Intensity_Decal _presetvalue_emissiveintensity))
        (`MaterialInstanceDynamic.SetScalarParameterValue` _returnvalue_3 "Scale_U" (.y (`SceneComponent.RelativeScale3D` _array_element)))
        (`MaterialInstanceDynamic.SetScalarParameterValue` _returnvalue_3 "Scale_V" (.z (`SceneComponent.RelativeScale3D` _array_element)))
        (`MaterialInstanceDynamic.SetScalarParameterValue` _returnvalue_3 "Lenght" Lenght)
        (else
          (`SceneComponent.SetVisibility` _array_element `Turn OF Decal` false)
          (`SceneComponent.SetRelativeScale3D` _array_element (0.0 0.0 0.0)))))))

(fn `UserConstructionScript`
  (bind (_presetvalue_presetname _presetvalue_intensity _presetvalue_lightcolor _presetvalue_attenuationradius _presetvalue_temperature _presetvalue_emissivecolor _presetvalue_emissivebrightness _presetvalue_emissivepower _presetvalue_lightbeamcolor _presetvalue_lightbeambrightness _presetvalue_lightbeampower) (break `/Game/_STALKER2/GameDesign/InteractiveObjects/LightBulb/DT_LightPresets/S_LightPresset` (`self.PresetValue`)))
  (bind (_presetvalue_presetname_2 _presetvalue_intensity_2 _presetvalue_lightcolor_2 _presetvalue_attenuationradius_2 _presetvalue_temperature_2) (break `/Game/_STALKER2/GameDesign/InteractiveObjects/LightBulb/DT_LightPresets/S_LightPresset` (`self.PresetValue`)))
  (bind (_presetvalue_presetname_3 _presetvalue_intensity_3 _presetvalue_lightcolor_3 _presetvalue_attenuationradius_3 _presetvalue_temperature_3 _presetvalue_emissivecolor_2 _presetvalue_emissivebrightness_2 _presetvalue_emissivepower_2 _presetvalue_lightbeamcolor_2 _presetvalue_lightbeambrightness_2 _presetvalue_lightbeampower_2 _presetvalue_emissiveintensity _presetvalue_glowcolor _presetvalue_glowintensity) (break `/Game/_STALKER2/GameDesign/InteractiveObjects/LightBulb/DT_LightPresets/S_LightPresset` (`self.PresetValue`)))
  (bind (_presetvalue_presetname_4 _presetvalue_intensity_4 _presetvalue_lightcolor_4 _presetvalue_attenuationradius_4 _presetvalue_temperature_4) (break `/Game/_STALKER2/GameDesign/InteractiveObjects/LightBulb/DT_LightPresets/S_LightPresset` (`self.PresetValue`)))
  (bind (_presetvalue_presetname_5 _presetvalue_intensity_5 _presetvalue_lightcolor_5 _presetvalue_attenuationradius_5 _presetvalue_temperature_5 _presetvalue_emissivecolor_3 _presetvalue_emissivebrightness_3 _presetvalue_emissivepower_3 _presetvalue_lightbeamcolor_3 _presetvalue_lightbeambrightness_3 _presetvalue_lightbeampower_3 _presetvalue_emissiveintensity_2 _presetvalue_glowcolor_2) (break `/Game/_STALKER2/GameDesign/InteractiveObjects/LightBulb/DT_LightPresets/S_LightPresset` (`self.PresetValue`)))
  (bind (_presetvalue_presetname_6 _presetvalue_intensity_6 _presetvalue_lightcolor_6 _presetvalue_attenuationradius_6 _presetvalue_temperature_6) (break `/Game/_STALKER2/GameDesign/InteractiveObjects/LightBulb/DT_LightPresets/S_LightPresset` (`self.PresetValue`)))
  (bind (_datatable _rowname) (break `DataTableRowHandle` (`self.LightingPresetColor`)))
  (bind (_datatable_2 _rowname_2) (break `DataTableRowHandle` (`self.LightingPresetRadius`)))
  (bind _returnvalue (!= _presetvalue_attenuationradius_6 0.0))
  (bind _returnvalue_2 (* _presetvalue_intensity_6 3.0))
  (bind _returnvalue_3 (* (`self.InnerIntensityMultiplier`) _presetvalue_intensity_2))
  (bind _returnvalue_4 (* _presetvalue_attenuationradius_6 3.0))
  (`parent.UserConstructionScript`)
  (`|ExecutionSequence`
    (:`then_0`
      ;[1 1 1] Get Values from DT
      (bind _returnvalue_5 (`|GetDataTableRow` _datatable _rowname)
        (:`then`
          (bind (_presetname _temperature _lightcolor _emissivecolor _lightbeamcolor _glowcolor) (break `/Game/_STALKER2/GameDesign/InteractiveObjects/LightBulb/DT_LightPresets/S_LightPresset_Color` _returnvalue_5))
          (set `self.PresetValue` (make `/Game/_STALKER2/GameDesign/InteractiveObjects/LightBulb/DT_LightPresets/S_LightPresset` "False" 0.0 _lightcolor 0.0 _temperature _emissivecolor 0.0 0.0 _lightbeamcolor 0.0 0.0 0.0 _glowcolor))
          (bind _returnvalue_6 (`|GetDataTableRow` _datatable_2 _rowname_2)
            (:`then`
              (bind (_presetname_2 _intensity _attenuationradius _emissivebrightness _emissivepower _lightbeambrightness _lightbeampower _emissiveintensity _glowintensity) (break `/Game/_STALKER2/GameDesign/InteractiveObjects/LightBulb/DT_LightPresets/S_LightPresset_Radius` _returnvalue_6))
              (set `self.PresetValue` (make `/Game/_STALKER2/GameDesign/InteractiveObjects/LightBulb/DT_LightPresets/S_LightPresset` "False" _intensity _presetvalue_lightcolor_5 _attenuationradius _presetvalue_temperature_5 _presetvalue_emissivecolor_3 _emissivebrightness _emissivepower _presetvalue_lightbeamcolor_3 _lightbeambrightness _lightbeampower _emissiveintensity _presetvalue_glowcolor_2 _glowintensity))
              (`|ExecutionSequence`
                (:`then_0`
                  ;[1 1 1] Point /Spot light
                  ;;[1 1 1] Intensity
                  (for _array_element (`self.PointLights`)
                    (`LocalLightComponent.SetIntensityUnits` _array_element "Lumens")
                    (`LightComponent.SetIntensity` _array_element _returnvalue_2)
                    ;;[1 1 1] Light color
                    (`LightComponent.SetLightColor` _array_element _presetvalue_lightcolor_6 true)
                    ;;[1 1 1] Temperature
                    (`LightComponent.SetTemperature` _array_element _presetvalue_temperature_6)
                    ;;[1 1 1] Attenuation Radius
                    (if _returnvalue
                      (`LocalLightComponent.SetAttenuationRadius` _array_element _returnvalue_4)))
                  (for _array_element_2 (`self.SpotLights`)
                    (`LocalLightComponent.SetIntensityUnits` _array_element_2 "Lumens")
                    (`LightComponent.SetIntensity` _array_element_2 _returnvalue_2)
                    (`LightComponent.SetLightColor` _array_element_2 _presetvalue_lightcolor_6 true)
                    (`LightComponent.SetTemperature` _array_element_2 _presetvalue_temperature_6)
                    (if _returnvalue
                      (`LocalLightComponent.SetAttenuationRadius` _array_element_2 _returnvalue_4)))
                  (set `self.BaseIntensity` _presetvalue_intensity_6))
                (:`then_1`
                  ;[0.3982 0.7647 1] SetupEmissive Array for Mesh with Glow
                  (`BlueprintMapLibrary.Map_Clear` (`self.GlowObjectsMaterialOrigin`))
                  (`BlueprintMapLibrary.Map_Clear` (`self.GlowObjectsMaterialNew`))
                  (`|ExecutionSequence`
                    (:`then_0`
                      ;;[1 1 1] Back Compatibility
                      (for _array_element_3 (`self.GetComponentsByTag` "/Script/Engine.StaticMeshComponent" "Glow")
                        (bind _returnvalue_7 (`PrimitiveComponent.GetMaterial` _array_element_3 0))
                        (`BlueprintMapLibrary.Map_Add` (`self.GlowObjectsMaterialOrigin`) _array_element_3 _returnvalue_7)
                        (bind _returnvalue_8 (`KismetMaterialLibrary.CreateDynamicMaterialInstance` _returnvalue_7))
                        (`MaterialInstanceDynamic.SetVectorParameterValue` _returnvalue_8 "EmissiveColor" _presetvalue_emissivecolor_2)
                        (`MaterialInstanceDynamic.SetScalarParameterValue` _returnvalue_8 "EmissiveMult" _presetvalue_emissivebrightness_2)
                        (`MaterialInstanceDynamic.SetScalarParameterValue` _returnvalue_8 "EmissivePower" _presetvalue_emissivepower_2)
                        (`BlueprintMapLibrary.Map_Add` (`self.GlowObjectsMaterialNew`) _array_element_3 _returnvalue_8)))
                    (:`then_1`
                      (for _array_element_4 (`self.GetComponentsByTag` "/Script/Engine.StaticMeshComponent" "EmissiveGlassOpaque")
                        (bind _returnvalue_9 (`PrimitiveComponent.GetMaterial` _array_element_4 0))
                        (`BlueprintMapLibrary.Map_Add` (`self.GlowObjectsMaterialOrigin`) _array_element_4 _returnvalue_9)
                        (bind _returnvalue_10 (`KismetMaterialLibrary.CreateDynamicMaterialInstance` _returnvalue_9))
                        (`MaterialInstanceDynamic.SetVectorParameterValue` _returnvalue_10 "EmissiveColor" _presetvalue_emissivecolor_2)
                        (`MaterialInstanceDynamic.SetScalarParameterValue` _returnvalue_10 "EmissiveIntensity" _presetvalue_emissiveintensity)
                        (`BlueprintMapLibrary.Map_Add` (`self.GlowObjectsMaterialNew`) _array_element_4 _returnvalue_10)))
                    (:`then_2`
                      (for _array_element_5 (`self.GetComponentsByTag` "/Script/Engine.StaticMeshComponent" "EmissiveGlow")
                        (bind _returnvalue_11 (`PrimitiveComponent.GetMaterial` _array_element_5 0))
                        (`BlueprintMapLibrary.Map_Add` (`self.GlowObjectsMaterialOrigin`) _array_element_5 _returnvalue_11)
                        (bind _returnvalue_12 (`KismetMaterialLibrary.CreateDynamicMaterialInstance` _returnvalue_11))
                        (`MaterialInstanceDynamic.SetVectorParameterValue` _returnvalue_12 "GlowColor" _presetvalue_glowcolor)
                        (`MaterialInstanceDynamic.SetScalarParameterValue` _returnvalue_12 "GlowIntensity" _presetvalue_glowintensity)
                        (`BlueprintMapLibrary.Map_Add` (`self.GlowObjectsMaterialNew`) _array_element_5 _returnvalue_12)))))
                (:`then_2`
                  ;[1 1 1] Setup LightBeam
                  (`KismetArrayLibrary.Array_Clear` (`self.LightBeamsDIM`))
                  (for _array_element_6 (`self.GetComponentsByTag` "/Script/Engine.StaticMeshComponent" "LightBeam")
                    (bind _returnvalue_13 (`KismetMaterialLibrary.CreateDynamicMaterialInstance` (`PrimitiveComponent.GetMaterial` _array_element_6 0)))
                    (`KismetArrayLibrary.Array_Add` (`self.LightBeamsDIM`) _returnvalue_13)
                    (`MaterialInstanceDynamic.SetVectorParameterValue` _returnvalue_13 "LightBeamColor" _presetvalue_lightbeamcolor)
                    (`MaterialInstanceDynamic.SetScalarParameterValue` _returnvalue_13 "LightBeamMult" _presetvalue_lightbeambrightness)
                    (`MaterialInstanceDynamic.SetScalarParameterValue` _returnvalue_13 "LightBeamPower" _presetvalue_lightbeampower)
                    (`PrimitiveComponent.SetMaterial` _array_element_6 0 _returnvalue_13)))
                (:`then_3`
                  ;[1 1 1] Inner Point /Spot light
                  ;;[1 1 1] Intensity
                  (for _array_element_7 (`self.InnerPointLights`)
                    (`LocalLightComponent.SetIntensityUnits` _array_element_7 "Lumens")
                    (`LightComponent.SetIntensity` _array_element_7 _returnvalue_3)
                    ;;[1 1 1] Light color
                    (`LightComponent.SetLightColor` _array_element_7 _presetvalue_lightcolor_2 true)
                    ;;[1 1 1] Temperature
                    (`LightComponent.SetTemperature` _array_element_7 _presetvalue_temperature_2))
                  (for _array_element_8 (`self.InnerSpotLights`)
                    (`LocalLightComponent.SetIntensityUnits` _array_element_8 "Lumens")
                    (`LightComponent.SetIntensity` _array_element_8 _returnvalue_3)
                    (`LightComponent.SetLightColor` _array_element_8 _presetvalue_lightcolor_2 true)
                    (`LightComponent.SetTemperature` _array_element_8 _presetvalue_temperature_2)))
                (:`then_4`
                  ;[1 1 1] Outer Point /Spot light
                  ;;[1 1 1] Intensity
                  (for _array_element_9 (`self.OuterPointLights`)
                    (`LocalLightComponent.SetIntensityUnits` _array_element_9 "Lumens")
                    (`LightComponent.SetIntensity` _array_element_9 _presetvalue_intensity_4)
                    ;;[1 1 1] Light color
                    (`LightComponent.SetLightColor` _array_element_9 _presetvalue_lightcolor_4 true)
                    ;;[1 1 1] Temperature
                    (`LightComponent.SetTemperature` _array_element_9 _presetvalue_temperature_4))
                  (for _array_element_10 (`self.OuterSpotLights`)
                    (`LocalLightComponent.SetIntensityUnits` _array_element_10 "Lumens")
                    (`LightComponent.SetIntensity` _array_element_10 _presetvalue_intensity_4)
                    (`LightComponent.SetLightColor` _array_element_10 _presetvalue_lightcolor_4 true)
                    (`LightComponent.SetTemperature` _array_element_10 _presetvalue_temperature_4)))
                (:`then_5`
                  (`self.OnConstruction_Child`))))
            (:`RowNotFound`
              (`KismetSystemLibrary.PrintString` "PresetSelectFail!" :!label _label))))
        (:`RowNotFound`
          (goto _label))))
    (:`then_1`
      ;[1 1 1] Projector LookAt Horizontal/Vertical
      (for _array_element_11 (`self.GetComponentsByTag` "/Script/Engine.StaticMeshComponent" "BaseH")
        (`SceneComponent.K2_SetRelativeRotation` _array_element_11 (`KismetMathLibrary.MakeRotator` 0.0 0.0 (`self.ProjectorH`)) false false))
      (for _array_element_12 (`self.GetComponentsByTag` "/Script/Engine.StaticMeshComponent" "BaseV")
        (`SceneComponent.K2_SetRelativeRotation` _array_element_12 (`KismetMathLibrary.MakeRotator` (`self.ProjctorV`)) false false)))))