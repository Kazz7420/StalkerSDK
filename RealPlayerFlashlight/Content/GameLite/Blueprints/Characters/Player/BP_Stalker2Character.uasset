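; BP_Stalker2Character is a player character Blueprint that adds a forward push to jumps and a hotkey for teleporting.
; On jump, a moving character is launched along the capsule's forward vector, with a stronger impulse when IsWalking is true than otherwise.
; The 0 key runs the XTeleport console command, noted as the global map teleport menu.
; An author comment flags the jump force as needing replication in code.
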(event `self.OnJumped`
  (bind (_returnvalue_x _returnvalue_y) (`KismetMathLibrary.BreakVector` (* (`SceneComponent.GetForwardVector` (`self.CapsuleComponent`)) 220.0)))
  (bind (_returnvalue_x_2 _returnvalue_y_2) (`KismetMathLibrary.BreakVector` (* (`SceneComponent.GetForwardVector` (`self.CapsuleComponent`)) 125.0)))
  ;[1 0 0.031] JumpForwardForce This need replicate in code
  (if (`CppMediator.IsMoving` self)
    (if (`CppMediator.IsWalking` self)
      (`self.LaunchCharacter` (`KismetMathLibrary.MakeVector` _returnvalue_x _returnvalue_y 1.0))
      (else
        (`self.LaunchCharacter` (`KismetMathLibrary.MakeVector` _returnvalue_x_2 _returnvalue_y_2 1.0))))))

(event `Key|Zero`
  (params (Key :type "Key Structure"))
  ;[1 1 1] Teleporting Menu (GlobalMap)
  (:`Pressed`
    (`KismetSystemLibrary.ExecuteConsoleCommand` "XTeleport" null)))

(fn `UserConstructionScript`)