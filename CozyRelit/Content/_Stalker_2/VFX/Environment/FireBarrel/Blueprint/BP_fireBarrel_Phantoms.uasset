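; Fire barrel environment Blueprint (Phantoms variant) that starts a looping fire sound through Wwise on BeginPlay.
; A light flicker graph is present but never runs: two randomly offset, restarting timelines would sum their coefficients to scale the barrel and main light intensities.
; The construction script is empty, and the three switch helper graphs hold only unused nested-Lerp selection nodes.
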(event `self.ReceiveBeginPlay`
  (`AkGameObject.PostAkEvent` :`self` (`self.Ak`) :`AkEvent` "/Game/_STALKER2/Audio/WwiseAudio/Events/EnvironmentParticles/Fire/SFX_Fire_Barrel_Loop.SFX_Fire_Barrel_Loop"))

(fn `UserConstructionScript`
  (locals (Niagara_s :type "NiagaraComponent Object Reference")))