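; BP_fireBarrel is an environmental burning barrel with looping fire audio, a moving light and a burn hazard.
; On BeginPlay it starts the sound and caches the main light's position, which Tick offsets with time-driven Perlin noise to fake firelight wobble.
; Its trigger applies effects to a BP_Stalker2Character on overlap and removes them on exit.
; The timeline-based intensity flicker is disconnected and never runs.
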(event `self.ReceiveBeginPlay`
  (`AkGameObject.PostAkEvent` :`self` (`self.Ak`) :`AkEvent` "/Game/_STALKER2/Audio/WwiseAudio/Events/EnvironmentParticles/Fire/SFX_Fire_Barrel_Loop.SFX_Fire_Barrel_Loop")
  (set `self.Light_Loc` (`SceneComponent.RelativeLocation` (`self.MainLight`))))

(event `self.ReceiveTick`
  (params (DeltaSeconds :type "Float (single-precision)"))
  (bind _lightwiggleh_int (`self.LightWiggleH_Int`))
  (bind _returnvalue (* (`KismetSystemLibrary.GetGameTimeInSeconds`) (`self.LightWiggle_Speed`)))
  (`SceneComponent.K2_SetRelativeLocation` (`self.MainLight`) (+ (`self.Light_Loc`) (`KismetMathLibrary.MakeVector` (* (`KismetAnimationLibrary.K2_MakePerlinNoiseAndRemap` (+ _returnvalue 25.0) -1.0 1.0) _lightwiggleh_int) (* (`KismetAnimationLibrary.K2_MakePerlinNoiseAndRemap` (+ _returnvalue 50.0) -1.0 1.0) _lightwiggleh_int) (* (`KismetAnimationLibrary.K2_MakePerlinNoiseAndRemap` (+ _returnvalue 100.0) -1.0 1.0) (`self.LightWiggleV_Int`)))) false false))

(event `self.BurnTriggerCollider.OnComponentBeginOverlap`
  (params (OverlappedComponent :type "PrimitiveComponent Object Reference") (OtherActor :type "Actor Object Reference") (OtherComp :type "PrimitiveComponent Object Reference") (OtherBodyIndex :type Integer) (bFromSweep :type Boolean) (SweepResult :type "HitResult Structure (by ref)"))
  ;[1 1 1] Apply / Remove Burning effect when player steps into the Fire
  (bind _asbp_stalker_2character (cast `/Game/GameLite/Blueprints/Characters/Player/BP_Stalker2Character` OtherActor))
  (`/Engine/EditorBlueprintResources/StandardMacros.IsValid` _asbp_stalker_2character
    (:`Is Valid`
      (`ApplyEffectComponent.ApplyEffects` (`self.ApplyEffect`) null))))

(event `self.BurnTriggerCollider.OnComponentEndOverlap`
  (params (OverlappedComponent :type "PrimitiveComponent Object Reference") (OtherActor :type "Actor Object Reference") (OtherComp :type "PrimitiveComponent Object Reference") (OtherBodyIndex :type Integer))
  ;[1 1 1] Apply / Remove Burning effect when player steps into the Fire
  (bind _asbp_stalker_2character (cast `/Game/GameLite/Blueprints/Characters/Player/BP_Stalker2Character` OtherActor))
  (`/Engine/EditorBlueprintResources/StandardMacros.IsValid` _asbp_stalker_2character
    (:`Is Valid`
      (`ApplyEffectComponent.RemoveEffects` (`self.ApplyEffect`) null))))

(fn `UserConstructionScript`
  (locals (Niagara_s :type "NiagaraComponent Object Reference")))