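; Campfire actor that plays a looping fire sound and burns the player who steps into it.
; BeginPlay posts the Wwise campfire loop, and BurnTriggerCollider overlaps apply or remove effects on BP_Stalker2Character through the ApplyEffect component.
; A two-timeline light flicker with random start offsets for the main and inner lights is present but never runs, and the switch helper functions are unused.
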(event `self.ReceiveBeginPlay`
  (`AkGameObject.PostAkEvent` :`self` (`self.Ak`) :`AkEvent` "/Game/_STALKER2/Audio/WwiseAudio/Events/EnvironmentParticles/Fire/SFX_Fire_Campfire_Loop.SFX_Fire_Campfire_Loop"))

(event `self.BurnTriggerCollider.OnComponentBeginOverlap`
  (params (OverlappedComponent :type "PrimitiveComponent Object Reference") (OtherActor :type "Actor Object Reference") (OtherComp :type "PrimitiveComponent Object Reference") (OtherBodyIndex :type Integer) (bFromSweep :type Boolean) (SweepResult :type "HitResult Structure (by ref)"))
  ;[1 1 1] Apply / Remove Burning effect when player steps into the Fire
  (bind _asbp_stalker_2character (cast `/Game/GameLite/Blueprints/Characters/Player/BP_Stalker2Character` OtherActor))
  (`/Engine/EditorBlueprintResources/StandardMacros.IsValid` _asbp_stalker_2character
    (:`Is Valid`
      (`ApplyEffectComponent.ApplyEffects` (`self.ApplyEffect`) null))))

(event `self.BurnTriggerCollider.OnComponentEndOverlap`
  (params (OverlappedComponent :type "PrimitiveComponent Object Reference") (OtherActor :type "Actor Object Reference") (OtherComp :type "PrimitiveComponent Object Reference") (OtherBodyIndex :type Integer))
  ;[1 1 1] Apply / Remove Burning effect when player steps into the Fire
  (bind _asbp_stalker_2character (cast `/Game/GameLite/Blueprints/Characters/Player/BP_Stalker2Character` OtherActor))
  (`/Engine/EditorBlueprintResources/StandardMacros.IsValid` _asbp_stalker_2character
    (:`Is Valid`
      (`ApplyEffectComponent.RemoveEffects` (`self.ApplyEffect`) null))))

(fn `UserConstructionScript`
  (locals (NS :type "NiagaraComponent Object Reference")))