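; Camp bonfire Blueprint that defines six seating spots, SitLocation0 through SitLocation5.
; The construction script derives each spot's world transform from a matching Arrow component, so moving an arrow sets the seat placement.
; Each transform keeps the arrow's location and scale, with yaw turned by -90 degrees and a height offset currently at zero.
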(fn `UserConstructionScript`
  (bind _returnvalue (`SceneComponent.K2_GetComponentToWorld` (`self.Arrow`)))
  (bind _returnvalue_2 (`SceneComponent.K2_GetComponentToWorld` (`self.Arrow1`)))
  (bind _returnvalue_3 (`SceneComponent.K2_GetComponentToWorld` (`self.Arrow2`)))
  (bind _returnvalue_4 (`SceneComponent.K2_GetComponentToWorld` (`self.Arrow3`)))
  (bind _returnvalue_5 (`SceneComponent.K2_GetComponentToWorld` (`self.Arrow5`)))
  (bind _returnvalue_6 (`SceneComponent.K2_GetComponentToWorld` (`self.Arrow4`)))
  (set `self.SitLocation_0` (`KismetMathLibrary.MakeTransform` (`KismetMathLibrary.MakeVector` (.x (.location _returnvalue)) (.y (.location _returnvalue)) (+ (.z (.location _returnvalue)) 0.0)) (`KismetMathLibrary.MakeRotator` (.roll (.rotation _returnvalue)) (.pitch (.rotation _returnvalue)) (+ (.yaw (.rotation _returnvalue)) -90.0)) (.scale _returnvalue)))
  (set `self.SitLocation_1` (`KismetMathLibrary.MakeTransform` (`KismetMathLibrary.MakeVector` (.x (.location _returnvalue_2)) (.y (.location _returnvalue_2)) (+ (.z (.location _returnvalue_2)) 0.0)) (`KismetMathLibrary.MakeRotator` (.roll (.rotation _returnvalue_2)) (.pitch (.rotation _returnvalue_2)) (+ (.yaw (.rotation _returnvalue_2)) -90.0)) (.scale _returnvalue_2)))
  (set `self.SitLocation_2` (`KismetMathLibrary.MakeTransform` (`KismetMathLibrary.MakeVector` (.x (.location _returnvalue_3)) (.y (.location _returnvalue_3)) (+ (.z (.location _returnvalue_3)) 0.0)) (`KismetMathLibrary.MakeRotator` (.roll (.rotation _returnvalue_3)) (.pitch (.rotation _returnvalue_3)) (+ (.yaw (.rotation _returnvalue_3)) -90.0)) (.scale _returnvalue_3)))
  (set `self.SitLocation_3` (`KismetMathLibrary.MakeTransform` (`KismetMathLibrary.MakeVector` (.x (.location _returnvalue_4)) (.y (.location _returnvalue_4)) (+ (.z (.location _returnvalue_4)) 0.0)) (`KismetMathLibrary.MakeRotator` (.roll (.rotation _returnvalue_4)) (.pitch (.rotation _returnvalue_4)) (+ (.yaw (.rotation _returnvalue_4)) -90.0)) (.scale _returnvalue_4)))
  (set `self.SitLocation_4` (`KismetMathLibrary.MakeTransform` (`KismetMathLibrary.MakeVector` (.x (.location _returnvalue_6)) (.y (.location _returnvalue_6)) (+ (.z (.location _returnvalue_6)) 0.0)) (`KismetMathLibrary.MakeRotator` (.roll (.rotation _returnvalue_6)) (.pitch (.rotation _returnvalue_6)) (+ (.yaw (.rotation _returnvalue_6)) -90.0)) (.scale _returnvalue_6)))
  (set `self.SitLocation_5` (`KismetMathLibrary.MakeTransform` (`KismetMathLibrary.MakeVector` (.x (.location _returnvalue_5)) (.y (.location _returnvalue_5)) (+ (.z (.location _returnvalue_5)) 0.0)) (`KismetMathLibrary.MakeRotator` (.roll (.rotation _returnvalue_5)) (.pitch (.rotation _returnvalue_5)) (+ (.yaw (.rotation _returnvalue_5)) -90.0)) (.scale _returnvalue_5))))