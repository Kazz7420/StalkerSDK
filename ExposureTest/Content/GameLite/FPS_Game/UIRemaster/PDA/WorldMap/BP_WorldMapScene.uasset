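; World map scene actor for the PDA, rendering a map mesh through an orthographic SceneCaptureComponent2D into a render target.
; UI pan and zoom convert into capture offset and ortho width, and capture-every-frame is switchable.
; Mouse UV and unselected-area brightness feed the map's material parameters.
; An experimental WIP override alters WeatherController post-process settings one second after BeginPlay and restores the saved settings on EndPlay.
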(event `self.SetOffset`
  (params (InOffset :type "Vector2D Structure"))
  (bind (_x _y) (`KismetMathLibrary.BreakVector2D` InOffset))
  (`SceneComponent.K2_SetRelativeLocation` (`self.SceneCaptureComponent2D`) (`KismetMathLibrary.MakeVector` 0.0 (* _y -0.1) (* _x -0.1)) false false))

(event `self.SetScale`
  (params (InScale :type "Float (single-precision)"))
  (set `SceneCaptureComponent2D.OrthoWidth` (* (/ (`TextureRenderTarget2D.SizeX` (`SceneCaptureComponent2D.TextureTarget` (`self.SceneCaptureComponent2D`))) InScale) 0.1) (`self.SceneCaptureComponent2D`)))

(event `self.SetCaptureEveryFrame`
  (params (bIsEnabled :type Boolean))
  (set `SceneCaptureComponent.bCaptureEveryFrame` bIsEnabled (`self.SceneCaptureComponent2D`)))

(event `self.SetMouseUV`
  (params (InUV :type "Vector Structure"))
  (`MeshComponent.SetVectorParameterValueOnMaterials` (`self.Map`) "Position" InUV))

(event `self.SetNotSelectedAreaBrightness`
  (params (InBrightness :type "Float (single-precision)"))
  (`MeshComponent.SetScalarParameterValueOnMaterials` (`self.Map`) "NotSelectedAreaBrightnes" InBrightness))

(event `self.ReceiveBeginPlay`
  ;[1 1 1] Experimental PP Set WIP
  ;;[1 1 1] Wait to make sure Weather is loaded
  (`KismetSystemLibrary.Delay` 1.0)
  (bind _outactors (`GameplayStatics.GetAllActorsOfClass` "/Game/light/WeatherController_BP.WeatherController_BP_C"))
  (for _array_element _outactors
    (bind _settings (`PostProcessComponent.Settings` (`self.GetComponentByClass` _array_element "/Script/Engine.PostProcessComponent")))
    (set `self.PPDefaults` _settings)
    (setmembers `PostProcessSettings` :`StructRef` _settings :`TemperatureType` "TEMP_ColorTemperature" :`WhiteTemp` 6800.0 :`ColorCorrectionHighlightsMin` -0.045 :`BloomIntensity` 0.45 :`AmbientCubemapIntensity` 0.015 :`AutoExposureMeterMask` "/Game/light/textures/Exposure_T_EV_Mask_Linear.Exposure_T_EV_Mask_Linear" :`AutoExposureSpeedUp` 10.0 :`AutoExposureSpeedDown` 14.0 :`LocalExposureHighlightContrastScale` 0.6 :`LocalExposureBlurredLuminanceBlend` 0.5 :`LocalExposureBlurredLuminanceKernelSizePercent` 50.0 :`LocalExposureMiddleGreyBias` -0.3 :`AmbientOcclusionIntensity` 0.75 :`AmbientOcclusionRadius` 200.0 :`AmbientOcclusionPower` 2.0)))

(event `self.ReceiveEndPlay`
  (params (EndPlayReason :type "EEndPlayReason Enum" :default "Destroyed"))
  ;[1 1 1] Experimental PP Set WIP
  (bind _outactors (`GameplayStatics.GetAllActorsOfClass` "/Game/light/WeatherController_BP.WeatherController_BP_C"))
  (for _array_element _outactors
    (set `PostProcessComponent.Settings` (`self.PPDefaults`) (`self.GetComponentByClass` _array_element "/Script/Engine.PostProcessComponent"))))

(fn `UserConstructionScript`)